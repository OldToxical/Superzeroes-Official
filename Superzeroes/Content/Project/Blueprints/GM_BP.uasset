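; GM_BP is a game mode Blueprint that spawns the player character when play begins.
; BeginPlay calls SpawnPlayers, which spawns a BoomBoom_BP high above the world origin and has player controller 0 possess it.
; An unconnected chain would add a second local player possessing ZipZap_BP, destroy existing camera actors and point both controllers at a SetSceneCamera_BP view, but it never runs.
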(event `self.ReceiveBeginPlay`
  (`self.SpawnPlayers`))

(fn `SpawnPlayers`
  (bind _returnvalue (`|SpawnActorFromClass` "/Game/Project/Blueprints/Superzeroes/BoomBoom_BP.BoomBoom_BP_C" (`KismetMathLibrary.MakeTransform` (0.0 0.0 2000.0)) "AlwaysSpawn" "OverrideRootScale" null 0 null))
  (`Controller.Possess` (`GameplayStatics.GetPlayerController` 0) _returnvalue))

(fn `UserConstructionScript`)