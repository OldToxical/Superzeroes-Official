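; ZipZap_BP is the ZipZap Superzeroes player actor, handling spawn placement and HUD setup at BeginPlay.
; SpawnFunction teleports it to the PlayerStart whose tag is "player" plus its PlayerInt.
; BeginPlay also adds a ZZ_Bars_BP widget, caches its Niagara widgets for combo, health and level-finished effects, and stores smoke and siege particle references, deactivating the siege one.
; Damage handling is unimplemented, with only an unconnected health clamp.
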(event `self.ReceiveBeginPlay`
  (`self.Spawn Function`)
  (bind _returnvalue (`|CreateWidget` "/Game/Project/Blueprints/UI/PlayerBars/ZZ_Bars_BP.ZZ_Bars_BP_C"))
  (`UserWidget.AddToViewport` _returnvalue 0)
  (set `self.smokeParticle` (`self.Niagara`))
  (set `self.comboBarParticle` (`/Game/Project/Blueprints/UI/PlayerBars/ZZ_Bars_BP.NiagaraSystemWidget_0` _returnvalue))
  (set `self.levelFinishedParticle` (`/Game/Project/Blueprints/UI/PlayerBars/ZZ_Bars_BP.NiagaraSystemWidget_3` _returnvalue))
  (set `self.healthBarParticle` (`/Game/Project/Blueprints/UI/PlayerBars/ZZ_Bars_BP.NiagaraSystemWidget_1` _returnvalue))
  (bind _output_get (set `self.siegeInitiationParticle` (`self.Siege_Ini_Particle`)))
  (`ActorComponent.Deactivate` _output_get))

(event `self.ReceiveTick`
  (params (DeltaSeconds :type "Float (single-precision)")))

(event `self.ReceiveAnyDamage`
  (params (Damage :type "Float (single-precision)") (DamageType :type "DamageType Object Reference") (InstigatedBy :type "Controller Object Reference") (DamageCauser :type "Actor Object Reference")))

(fn `Spawn Function`
  (bind _outactors (`GameplayStatics.GetAllActorsOfClass` "/Script/Engine.PlayerStart"))
  (for _array_element _outactors
    (if (== (`PlayerStart.PlayerStartTag` _array_element) (`KismetStringLibrary.Concat_StrStr` "player" (`KismetStringLibrary.Conv_IntToString` (`self.PlayerInt`))))
      (`self.K2_SetActorLocation` (`self.K2_GetActorLocation` _array_element) false true))))

(fn `UserConstructionScript`)