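; BoomBoom is a Superzero actor that sets up its own spawn and HUD and brings the second player, ZipZap, into the game.
; On BeginPlay it moves to the PlayerStart tagged with its player number, creates the bars widget and caches Niagara effect references.
; When CanSpawnZipZap is set, Tick creates a second local player possessing ZipZap, destroys CameraActors and points both controllers at the shared scene camera.
; Reset reloads Sample2DLevel; ZipZap input and damage handlers are empty.
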(event `self.ReceiveBeginPlay`
  (`self.Spawn Function`)
  (set `self.smokeParticle` (`self.Niagara`))
  (bind _returnvalue (`|CreateWidget` "/Game/Project/Blueprints/UI/PlayerBars/BB_Bars_BP.BB_Bars_BP_C"))
  (`UserWidget.AddToViewport` _returnvalue 0)
  (set `self.comboBarParticle` (`/Game/Project/Blueprints/UI/PlayerBars/BB_Bars_BP.NiagaraSystemWidget_128` _returnvalue))
  (set `self.levelFinishedParticle` (`/Game/Project/Blueprints/UI/PlayerBars/BB_Bars_BP.NiagaraSystemWidget_11` _returnvalue))
  (bind _output_get (set `self.siegeInitiationParticle` (`self.Siege_Ini_Particle`)))
  (`ActorComponent.Deactivate` _output_get))

(event `self.ReceiveTick`
  (params (DeltaSeconds :type "Float (single-precision)"))
  (if (`self.canSpawnZipZap`)
    (`self.Spawn ZZ`)))

(event `self.ReceiveAnyDamage`
  (params (Damage :type "Float (single-precision)") (DamageType :type "DamageType Object Reference") (InstigatedBy :type "Controller Object Reference") (DamageCauser :type "Actor Object Reference")))

(event `InputAction|Reset scene`
  (params (Key :type "Key Structure"))
  (:`Pressed`
    (`GameplayStatics.OpenLevel` "Sample2DLevel")))

(event `InputAxis|MoveZipZap`
  (params (AxisValue :type "Float (single-precision)")))

(event `InputAction|ShootZipZap`
  (params (Key :type "Key Structure")))

(event `InputAction|JumpZipZap`
  (params (Key :type "Key Structure")))

(event `InputAxis|ClimbZipZap`
  (params (AxisValue :type "Float (single-precision)")))

(event `InputAction|InitiateComboAttack_Savage`
  (params (Key :type "Key Structure")))

(fn `Spawn Function`
  (bind _outactors (`GameplayStatics.GetAllActorsOfClass` "/Script/Engine.PlayerStart"))
  (for _array_element _outactors
    (if (== (`PlayerStart.PlayerStartTag` _array_element) (`KismetStringLibrary.Concat_StrStr` "player" (`KismetStringLibrary.Conv_IntToString` (`self.PlayerInt`))))
      (`self.K2_SetActorLocation` (`self.K2_GetActorLocation` _array_element) false true))))

(fn `Spawn ZZ`
  (bind _returnvalue (`GameplayStatics.GetPlayerController` 1))
  (`GameplayStatics.CreatePlayer` 1)
  (bind _returnvalue_2 (`|SpawnActorFromClass` "/Game/Project/Blueprints/Superzeroes/ZipZap_BP.ZipZap_BP_C" (`KismetMathLibrary.MakeTransform` (+ (`self.K2_GetActorLocation`) (150.0 0.0 0.0))) "Undefined" "OverrideRootScale" null 1 null))
  (`Controller.Possess` _returnvalue _returnvalue_2)
  (bind _outactors (`GameplayStatics.GetAllActorsOfClass` "/Script/Engine.CameraActor"))
  (for _array_element _outactors
    (`self.K2_DestroyActor` _array_element))
  (bind _outactors_2 (`GameplayStatics.GetAllActorsOfClass` "/Game/Project/Blueprints/SetSceneCamera_BP.SetSceneCamera_BP_C"))
  (`PlayerController.SetViewTargetWithBlend` _returnvalue (`|GetArrayItem` _outactors_2) 0.0 "VTBlend_Linear" 0.0 false)
  (`PlayerController.SetViewTargetWithBlend` (`GameplayStatics.GetPlayerController` 0) (`|GetArrayItem` _outactors_2) 0.0 "VTBlend_Linear" 0.0 false)
  (set `self.canSpawnZipZap` false))

(fn `UserConstructionScript`)