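; Camera_BP is a shared camera rig meant to frame two players, the ZipZap and BoomBoom actors.
; BeginPlay caches the first actor of each class as P1 and P2.
; Disconnected logic would center the root slightly above their midpoint and set spring arm length to their distance, clamped to a minimum.
; Tick is empty, so the camera does not currently follow or zoom.
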(event `self.ReceiveBeginPlay`
  (bind _outactors (`GameplayStatics.GetAllActorsOfClass` "/Script/Superzeroes.ZipZap"))
  (set `self.P1` (`|GetArrayItem` _outactors))
  (bind _outactors_2 (`GameplayStatics.GetAllActorsOfClass` "/Script/Superzeroes.BoomBoom"))
  (set `self.P2` (`|GetArrayItem` _outactors_2)))

(event `self.ReceiveTick`
  (params (DeltaSeconds :type "Float (single-precision)")))

(fn `Get Distance Between Players`
  (returns (ReturnValue :type "Float (double-precision)"))
  (return (`KismetMathLibrary.FMax` (`KismetMathLibrary.VSize` (- (`self.K2_GetActorLocation` (`self.P1`)) (`self.K2_GetActorLocation` (`self.P2`)))) 200.0)))

(fn `UserConstructionScript`)