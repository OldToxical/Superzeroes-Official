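; DynamicCamera_BP is a shared dynamic camera rig that frames two player characters, ZipZap and BoomBoom.
; BeginPlay caches the first actor found of each class as P1 and P2.
; Every Tick moves the root to their midpoint with a zero-duration MoveComponentTo.
; It also sets the spring arm length from their separation, with a minimum distance and added padding, so the view zooms as they spread apart.
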(event `self.ReceiveBeginPlay`
  (bind _outactors (`GameplayStatics.GetAllActorsOfClass` "/Script/Superzeroes.ZipZap"))
  (set `self.P1` (`|GetArrayItem` _outactors))
  (bind _outactors_2 (`GameplayStatics.GetAllActorsOfClass` "/Script/Superzeroes.BoomBoom"))
  (set `self.P2` (`|GetArrayItem` _outactors_2)))

(event `self.ReceiveTick`
  (params (DeltaSeconds :type "Float (single-precision)"))
  (`KismetSystemLibrary.MoveComponentTo` (`self.DefaultSceneRoot`) (/ (+ (`self.K2_GetActorLocation` (`self.P1`)) (`self.K2_GetActorLocation` (`self.P2`))) (2.0 2.0 2.0)) (struct) false false 0.0)
  (bind _returnvalue (`self.Get Distance Between Players`))
  (set `SpringArmComponent.TargetArmLength` _returnvalue (`self.SpringArm`)))

(fn `Get Distance Between Players`
  (returns (ReturnValue :type "Float (double-precision)"))
  (return (+ (`KismetMathLibrary.FMax` (`KismetMathLibrary.VSize` (- (`self.K2_GetActorLocation` (`self.P1`)) (`self.K2_GetActorLocation` (`self.P2`)))) 200.0) 100.0)))

(fn `UserConstructionScript`)