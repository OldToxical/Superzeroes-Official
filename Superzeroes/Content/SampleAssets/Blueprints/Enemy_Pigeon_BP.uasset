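; Pigeon enemy Blueprint that sets up references and forwards bullet and animation events to collision and attack functions defined outside this graph.
; On BeginPlay it caches the BoomBoom and ZipZap actors and its Flipbook component.
; Exported particle data is looped over, passing each position to ProcessBulletCollision, so particles act as bullets.
; When the flipbook finishes playing, it calls EndAttack.
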(event `self.ReceiveBeginPlay`
  (bind _returnvalue (`GameplayStatics.GetActorOfClass` "/Script/Superzeroes.BoomBoom"))
  (set `self.boomBoom` _returnvalue)
  (bind _returnvalue_2 (`GameplayStatics.GetActorOfClass` "/Script/Superzeroes.ZipZap"))
  (set `self.zipZap` _returnvalue_2)
  (set `self.flipbookComponent` (`self.Flipbook`)))

(event `self.ReceiveActorBeginOverlap`
  (params (OtherActor :type "Actor Object Reference")))

(event `self.ReceiveTick`
  (params (DeltaSeconds :type "Float (single-precision)")))

(event `self.ReceiveParticleData`
  (params (Data :type "Array of BasicParticleData Structure (by ref)") (NiagaraSystem :type "NiagaraSystem Object Reference") (SimulationPositionOffset :type "Vector Structure (by ref)"))
  (for _array_element Data
    (`self.ProcessBulletCollision` (`.Position` (break `BasicParticleData` _array_element)))))

(event `self.Flipbook.OnFinishedPlaying`
  (`self.EndAttack`))

(fn `UserConstructionScript`)