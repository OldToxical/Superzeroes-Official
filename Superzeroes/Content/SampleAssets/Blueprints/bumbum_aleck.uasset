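; Blueprint for the 2D flipbook actor bumbum_aleck, which has its own health bar and attack state.
; BeginPlay caches the ZipZap actor and smoke particle, then adds the BBHealthBar_BP widget to the viewport.
; The flipbook's finished event ends the attack, and the Reset scene input reopens Sample2DLevel.
; AnyDamage is empty, with a health-clamping node left unused.
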(event `self.ReceiveBeginPlay`
  (bind _returnvalue (`GameplayStatics.GetActorOfClass` "/Script/Superzeroes.ZipZap"))
  (set `self.zipZap` _returnvalue)
  (set `self.smokeParticle` (`self.P_Smoke`))
  (bind _returnvalue_2 (`|CreateWidget` "/Game/SampleAssets/Blueprints/HealthBars/BBHealthBar_BP.BBHealthBar_BP_C"))
  (`UserWidget.AddToViewport` _returnvalue_2 0)
  (`GameplayStatics.GetActorOfClass` null))

(event `self.flipbook.OnFinishedPlaying`
  (`self.EndAttack`))

(event `self.ReceiveAnyDamage`
  (params (Damage :type "Float (single-precision)") (DamageType :type "DamageType Object Reference") (InstigatedBy :type "Controller Object Reference") (DamageCauser :type "Actor Object Reference")))

(event `InputAction|Reset scene`
  (params (Key :type "Key Structure"))
  (:`Pressed`
    (`GameplayStatics.OpenLevel` "Sample2DLevel")))

(fn `UserConstructionScript`)